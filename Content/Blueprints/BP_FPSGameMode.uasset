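; BP_FPSGameMode is the game mode that handles the end-of-mission screen flow through its OnMissionComplete event.
; The event removes objective info widgets, then shows WBP_GameOver, whose Success input is fixed to false, and WBP_MissionMenu.
; It then switches the first player to UI-only input focused on the menu and shows the mouse cursor.
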(event EventBeginPlay)

(event EventTick
  (params (DeltaSeconds :type Float%20%28single-precision%29)))

(event EventOnMissionComplete
  (params (InstigatorPawn :type Pawn%20Object%20Reference) (bSuccess :type Boolean))
  (Utilities|FlowControl|Sequence
    (:then_0
      (bind _foundwidgets (Widget|GetAllWidgetsOfClass "/Game/UI/WBP_ObjectiveInfo.WBP_ObjectiveInfo_C" true))
      (Widget|RemovefromParent _foundwidgets))
    (:then_1
      (bind _returnvalue (UserInterface|CreateWidget "/Game/UI/WBP_GameOver.WBP_GameOver_C"))
      (UserInterface|Viewport|AddtoViewport _returnvalue 0))
    (:then_2
      (bind _returnvalue_2 (UserInterface|CreateWidget "/Game/UI/WBP_MissionMenu.WBP_MissionMenu_C" (Game|GetPlayerController 0)))
      (UserInterface|Viewport|AddtoViewport _returnvalue_2 0)
      (Input|SetInputModeUIOnly (Game|GetPlayerController 0) _returnvalue_2 "DoNotLock")
      (Variables|/Script/Engine.PlayerController|SetbShowMouseCursor (Game|GetPlayerController 0) true))))

(fn ConstructionScript)